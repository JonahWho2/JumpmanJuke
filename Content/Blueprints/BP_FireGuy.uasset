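; BP_FireGuy is an actor that moves its Fire component endlessly back and forth between Start and End points.
; BeginPlay calls Loop, where a FlipFlop alternates a timeline between playing forward and in reverse, calling Loop again when it finishes.
; Each timeline update lerps Fire's world location without sweep and applies the Speed variable as play rate.
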(event Custom|Loop
  (Utilities|FlowControl|FlipFlop
    (:A
      (bind _newtrack_1 (Timeline|Timeline PlayFromStart)
        (:Update
          (Components|Timeline|SetPlayRate (Variables|Default|GetTimeline) (Variables|Default|Getspeed))
          (Transformation|SetWorldLocation (Variables|Default|GetFire) (Math|Vector|Lerp(Vector) (Transformation|GetWorldLocation (Variables|Default|GetStart)) (Transformation|GetWorldLocation (Variables|Default|GetEnd)) _newtrack_1) false false))
        (:Finished
          (CallFunction|Loop))))
    (:B
      (Timeline|Timeline ReverseFromEnd))))

(event EventBeginPlay
  (CallFunction|Loop))

(fn ConstructionScript)