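; Barrel spawner actor that keeps spawning BP_Barrel actors at random points for as long as it is in play.
; Each spawn uses the world transform of a randomly picked direct child component of DefaultSceneRoot, so those child components act as the spawn points.
; A custom event starts on BeginPlay and re-calls itself after a random delay of one to three seconds, forming an endless loop.
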(event Custom|SpawnBarrel
  (Game|SpawnActorfromClass "/Game/Blueprints/BP_Barrel.BP_Barrel_C" (Transformation|GetWorldTransform (.OutItem (Utilities|Array|Random (Components|GetChildrenComponents (Variables|Default|GetDefaultSceneRoot) false)))) "Undefined" "MultiplyWithRoot" 0 0)
  (Utilities|FlowControl|Delay (Math|Float|Lerp 1.0 3.0 (Math|Random|RandomFloat)))
  (CallFunction|SpawnBarrel))

(event EventBeginPlay
  (CallFunction|SpawnBarrel))

(fn ConstructionScript)